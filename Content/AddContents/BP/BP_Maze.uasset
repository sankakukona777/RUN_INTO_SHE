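; BP_Maze is an actor that builds a seeded grid maze at construction, placing a Hierarchical Instanced Static Mesh instance on each path tile.
; GenerateMaze uses randomized depth-first carving: AddNeighbourLoc recursively steps two cells in valid directions, recording bridge cells and single-neighbour dead ends.
; Backtrack pops ToCheck and moves bridge cells into the path until none remain.
; An author note marks GenerateMaze as not working; debug prints remain.
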(event EventBeginPlay)

(event Collision|EventActorBeginOverlap
  (params (OtherActor :type Actor%20Object%20Reference)))

(event EventTick
  (params (DeltaSeconds :type Float%20%28single-precision%29)))

(fn ConstructionScript
  (bind _tilesize (Variables|Default|GetTileSize))
  (bind _pathtilesout (CallFunction|GenerateMaze (Variables|Default|GetSeed) (Variables|Default|GetSize)))
  (bind _result (Utilities|Set|ToArray _pathtilesout))
  (for _array_element _result
    (Development|PrintString "Hello")
    (Components|InstancedStaticMesh|AddInstance (Variables|Default|GetHierarchicalInstancedStaticMesh) (Math|Transform|MakeTransform (Math|Vector|MakeVector (* (.X (Utilities|Struct|BreakIntPoint _array_element)) _tilesize) (* (.Y (Utilities|Struct|BreakIntPoint _array_element)) _tilesize) 0.0)))
    (Development|PrintString "Maze Generated")))

(fn GenerateMaze
  (params (Seed :type Integer) (Size :type Int%20Point%20Structure))
  (Math|Random|SetRandomStreamSeed (LocalVariables|GetRandStream) Seed)
  (Variables|Default|SetSize Size)
  (bind _output_get (LocalVariables|SetStartingLoc (Utilities|GetRandLocinBounds (LocalVariables|GetL_Size) (LocalVariables|GetRandStream))))
  (LocalVariables|SetCurrentLocation _output_get)
  (CallFunction|AddNeighbourLoc (LocalVariables|GetL_Size) (LocalVariables|GetRandStream) (LocalVariables|GetCurrentLocation) (LocalVariables|GetPathTiles) (LocalVariables|GetBridgeTiles) (LocalVariables|GetToCheck) (LocalVariables|GetEndPaths) :!label _label)
  (if (> (Utilities|Set|Length (LocalVariables|GetToCheck)) 0)
    (CallFunction|Backtrack (LocalVariables|GetCurrentLocation) (LocalVariables|GetToCheck) (LocalVariables|GetBridgeTiles) (LocalVariables|GetPathTiles))
    (goto _label)
    (else
      (return (LocalVariables|GetPathTiles) (LocalVariables|GetEndPaths)))))

(fn AddNeighbourLoc
  (params (Size :type Int%20Point%20Structure%20%28by%20ref%29) (RandStream :type Random%20Stream%20Structure%20%28by%20ref%29) (CurrentLoc :type Int%20Point%20Structure%20%28by%20ref%29) (PathTiles :type Set%20of%20Int%20Point%20Structures) (BridgeTiles :type Set%20of%20Int%20Point%20Structures) (ToCheck :type Set%20of%20Int%20Point%20Structures) (EndPaths :type Set%20of%20Int%20Point%20Structures))
  (LocalVariables|SetNeighbourIndex (Math|Random|RandomIntegerinRangefromStream 0 3 RandStream))
  (if (Utilities|CheckIsValidLoc (.Floor (Utilities|GetNeighbourandBridge CurrentLoc (LocalVariables|GetNeighbourIndex))) Size PathTiles BridgeTiles) :!label _label
    (Utilities|Set|Add PathTiles (.Floor (Utilities|GetNeighbourandBridge CurrentLoc (LocalVariables|GetNeighbourIndex))))
    (Utilities|Set|Add BridgeTiles (.Bridge (Utilities|GetNeighbourandBridge CurrentLoc (LocalVariables|GetNeighbourIndex))))
    (Utilities|Set|Add ToCheck (.Floor (Utilities|GetNeighbourandBridge CurrentLoc (LocalVariables|GetNeighbourIndex))))
    (CallFunction|AddNeighbourLoc Size RandStream (.Floor (Utilities|GetNeighbourandBridge CurrentLoc (LocalVariables|GetNeighbourIndex))) PathTiles BridgeTiles ToCheck EndPaths)
    (else
      (Utilities|DoN+ 4
        (:Exit
          (LocalVariables|SetNeighbourIndex (Math|Integer|SelectInt 0 (+ (LocalVariables|GetNeighbourIndex) 1) (>= (+ (LocalVariables|GetNeighbourIndex) 1) 4)))
          (goto _label))
        (:Over%20Nth
          (bind _count (CallFunction|GetNeighbourCount CurrentLoc PathTiles))
          (if (== _count 1)
            (Utilities|Set|Add EndPaths CurrentLoc)))))))

(fn GetNeighbourCount
  (params (CurrentLoc :type Int%20Point%20Structure%20%28by%20ref%29) (PathTiles :type Set%20of%20Int%20Point%20Structures))
  (for _array_element (Utilities|GetNeighborLoc CurrentLoc 1)
    (if (Utilities|Set|Contains PathTiles _array_element)
      (Math|Integer|IncrementInt (LocalVariables|GetCounter))))
  (return (LocalVariables|GetCounter)))

(fn Backtrack
  (params (CurrentTile :type Int%20Point%20Structure) (ToCheck :type Set%20of%20Int%20Point%20Structures) (BridgeTiles :type Set%20of%20Int%20Point%20Structures) (PathTiles :type Set%20of%20Int%20Point%20Structures))
  (bind _result (Utilities|Set|ToArray ToCheck))
  (|SetBy-RefVar CurrentTile (Utilities|Array|Get(acopy) _result (Utilities|Array|LastIndex _result)))
  (Utilities|Set|Remove ToCheck (Utilities|Array|Get(acopy) _result (Utilities|Array|LastIndex _result)))
  (bind _result_2 (Utilities|Set|ToArray BridgeTiles))
  (Utilities|Set|Add PathTiles (Utilities|Array|Get(acopy) _result_2 (Utilities|Array|LastIndex _result_2)))
  (Utilities|Set|Remove BridgeTiles (Utilities|Array|Get(acopy) _result_2 (Utilities|Array|LastIndex _result_2))))